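; BP_MeleePrefab is a melee enemy that tracks player proximity and handles its own damage and death.
; StopBox and AttackBox overlaps with the player's capsule toggle PlayerFound and AttackPlayer, apparently for the behavior tree.
; Damage drains Shield before Health, though damage exceeding Shield overwrites Health with the excess instead of subtracting it.
; Below zero Health, it decrements any assigned Wave's EnemyCount, plays an animation, disables collision and destroys itself after a delay.
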(event OnComponentBeginOverlap(StopBox)
  (params (OverlappedComponent :type Primitive%20Component%20Object%20Reference) (OtherActor :type Actor%20Object%20Reference) (OtherComp :type Primitive%20Component%20Object%20Reference) (OtherBodyIndex :type Integer) (bFromSweep :type Boolean) (SweepResult :type Hit%20Result%20Structure%20%28by%20ref%29))
  ;[0 1 0.9647] Tells the AI Behaviour Tree to fucking stop, and then summarily start again - Nathan
  (if (== OtherComp (Variables|/Script/Engine.Character|GetCapsuleComponent (.AsTop%20Down%20Character (Utilities|Casting|CastToTopDownCharacter (Game|GetPlayerCharacter 0)))))
    (Variables|Default|SetPlayerFound true)))

(event OnComponentEndOverlap(StopBox)
  (params (OverlappedComponent :type Primitive%20Component%20Object%20Reference) (OtherActor :type Actor%20Object%20Reference) (OtherComp :type Primitive%20Component%20Object%20Reference) (OtherBodyIndex :type Integer))
  ;[0 1 0.9647] Tells the AI Behaviour Tree to fucking stop, and then summarily start again - Nathan
  (if (== OtherComp (Variables|/Script/Engine.Character|GetCapsuleComponent (.AsTop%20Down%20Character (Utilities|Casting|CastToTopDownCharacter (Game|GetPlayerCharacter 0)))))
    (Variables|Default|SetPlayerFound false)))

(event OnComponentBeginOverlap(AttackBox)
  (params (OverlappedComponent :type Primitive%20Component%20Object%20Reference) (OtherActor :type Actor%20Object%20Reference) (OtherComp :type Primitive%20Component%20Object%20Reference) (OtherBodyIndex :type Integer) (bFromSweep :type Boolean) (SweepResult :type Hit%20Result%20Structure%20%28by%20ref%29))
  ;[0 1 0.9647] Checking if Player is in box - Nathan
  (if (== OtherComp (Variables|/Script/Engine.Character|GetCapsuleComponent (.AsTop%20Down%20Character (Utilities|Casting|CastToTopDownCharacter (Game|GetPlayerCharacter 0)))))
    (Variables|Default|SetAttack%20Player true)))

(event OnComponentEndOverlap(AttackBox)
  (params (OverlappedComponent :type Primitive%20Component%20Object%20Reference) (OtherActor :type Actor%20Object%20Reference) (OtherComp :type Primitive%20Component%20Object%20Reference) (OtherBodyIndex :type Integer))
  ;[0 1 0.9647] Checking if Player is in box - Nathan
  (if (== OtherComp (Variables|/Script/Engine.Character|GetCapsuleComponent (.AsTop%20Down%20Character (Utilities|Casting|CastToTopDownCharacter (Game|GetPlayerCharacter 0)))))
    (Variables|Default|SetAttack%20Player false)))

(event Custom|Enemy%20Wave
  (params (Wave :type BP%20Wave%20Spawner%20Object%20Reference))
  ;[0 1 0.9842] If the enemy is part of a Wave - Nathan
  (bind _output_get (Variables|Default|SetWave Wave)))

(event Game|Damage|EventAnyDamage
  (params (Damage :type Float%20%28single-precision%29) (DamageType :type Damage%20Type%20Object%20Reference) (InstigatedBy :type Controller%20Object%20Reference) (DamageCauser :type Actor%20Object%20Reference))
  (bind _returnvalue (Math|Float|Truncate Damage))
  ;[0 1 0.9647] Damage and Death Event - Nathan
  (if (> (Variables|Default|GetShield) 0)
    (if (> _returnvalue (Variables|Default|GetShield))
      (Variables|Default|SetHealth (- _returnvalue (Variables|Default|GetShield)))
      (Variables|Default|SetShield 0)
      (if (< (stale _output_get) 0) :!label _label
        (Variables|Default|GetWave
          (:then
            (Variables|/Game/AI/Spawners/BP_WaveSpawner.BP_WaveSpawner_C|SetEnemy%20Count (stale Custom|Enemy%20Wave _output_get) (- (Variables|/Game/AI/Spawners/BP_WaveSpawner.BP_WaveSpawner_C|GetEnemy%20Count (stale Custom|Enemy%20Wave _output_get)) 1)))
          (:else
            _))
        (Components|Animation|PlayAnimation (Variables|Character|GetMesh) "/Game/Mannequin/Animations/ThirdPersonJump_Loop.ThirdPersonJump_Loop" true)
        (Components|Movement|StopMovementImmediately (Variables|Character|GetCharacterMovement))
        (Collision|SetCollisionEnabled (Variables|Collision|GetCapsuleComponent) "NoCollision")
        (Utilities|FlowControl|Delay 2.0)
        (Actor|DestroyActor))
      (else
        (Variables|Default|SetShield (- (Variables|Default|GetShield) _returnvalue))))
    (else
      (bind _output_get (Variables|Default|SetHealth (- (Variables|Default|GetHealth) _returnvalue)))
      (goto _label))))

(fn ConstructionScript)