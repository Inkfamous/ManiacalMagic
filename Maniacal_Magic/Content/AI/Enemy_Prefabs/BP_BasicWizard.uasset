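; BP_BasicWizard is an AI wizard enemy that attacks by spawning Enemy_Fireball projectiles.
; Its FireProjectile event fires only when the Blackboard's PlayerSeen flag is true and TooClose is false.
; The fireball spawns at the capsule's location plus ProjectileOffset rotated into the capsule's orientation, and inherits the capsule's rotation.
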(event EventFireProjectile
  (bind _capsulecomponent (Variables|Default|GetCapsuleComponent))
  (bind _returnvalue (Transformation|GetWorldRotation _capsulecomponent))
  (if (ScalableFloat|GetValueasBool (AI|GetBlackboard self) (Utilities|Name|MakeLiteralName "PlayerSeen"))
    (if (not (Variables|Default|GetToo%20Close?))
      (Game|SpawnActorfromClass "/Game/TopDownBP/Blueprints/Enemy_Fireball.Enemy_Fireball_C" (Math|Transform|MakeTransform (+ (Transformation|GetWorldLocation _capsulecomponent) (Math|Vector|RotateVector (Variables|Default|GetProjectile%20Offset) _returnvalue)) _returnvalue) "Undefined" 0 0))))

(fn ConstructionScript
  (|CallParentFunction))