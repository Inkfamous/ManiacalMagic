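; Grand wizard boss enemy that registers with the game mode's boss list and enemy count and adds the player's boss components on spawn.
; Each tick a Camera-channel trace toward the player sets the "TooClose!" blackboard key from the hit distance, feeding its AI.
; Damage lowers health; on death it removes the boss components, drops the list's first entry rather than itself, decrements the count and destroys itself.
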(event EventBeginPlay
  (bind _returnvalue (Game|GetGameMode))
  (bind _astop_down_game_mode (Utilities|Casting|CastToTopDownGameMode _returnvalue))
  (Utilities|FlowControl|Sequence
    (:then_0
      (Utilities|Array|Add (Variables|/Game/TopDownBP/Blueprints/TopDownGameMode.TopDownGameMode_C|GetBossAI (.AsTop%20Down%20Game%20Mode (Utilities|Casting|CastToTopDownGameMode (Game|GetGameMode)))) self)
      (Default|AddBossComponents (.AsTop%20Down%20Character (Utilities|Casting|CastToTopDownCharacter (Game|GetPlayerCharacter 0)))))
    (:then_1
      (Variables|/Game/TopDownBP/Blueprints/TopDownGameMode.TopDownGameMode_C|SetEnemy%20Count _astop_down_game_mode (+ (Variables|/Game/TopDownBP/Blueprints/TopDownGameMode.TopDownGameMode_C|GetEnemy%20Count _astop_down_game_mode) 1)))))

(event Game|Damage|EventAnyDamage
  (params (Damage :type Float%20%28single-precision%29) (DamageType :type Damage%20Type%20Object%20Reference) (InstigatedBy :type Controller%20Object%20Reference) (DamageCauser :type Actor%20Object%20Reference))
  (bind _returnvalue (Game|GetGameMode))
  (bind _astop_down_game_mode (Utilities|Casting|CastToTopDownGameMode _returnvalue))
  (bind _output_get (Variables|Default|SetHealth (- (Variables|Default|GetHealth) (Math|Float|Truncate Damage))))
  (if (<= _output_get 0)
    (Default|RemoveBossComponents (.AsTop%20Down%20Character (Utilities|Casting|CastToTopDownCharacter (Game|GetPlayerCharacter 0))))
    (Utilities|Array|RemoveIndex (Variables|/Game/TopDownBP/Blueprints/TopDownGameMode.TopDownGameMode_C|GetBossAI _astop_down_game_mode))
    (Variables|/Game/TopDownBP/Blueprints/TopDownGameMode.TopDownGameMode_C|SetEnemy%20Count _astop_down_game_mode (- (Variables|/Game/TopDownBP/Blueprints/TopDownGameMode.TopDownGameMode_C|GetEnemy%20Count _astop_down_game_mode) 1))
    (Actor|DestroyActor)))

(event EventTick
  (params (DeltaSeconds :type Float%20%28single-precision%29))
  (bind _returnvalue (Utilities|Name|MakeLiteralName "TooClose!"))
  (bind _self self)
  (bind _returnvalue_2 (AI|GetAIController _self))
  (bind _returnvalue_3 (AI|GetBlackboard _returnvalue_2))
  (bind _outhit (Collision|LineTraceByChannel (Transformation|GetWorldLocation (Variables|Collision|GetCapsuleComponent)) (Transformation|GetWorldLocation (Variables|/Script/Engine.Character|GetCapsuleComponent (Game|GetPlayerCharacter 0))) "TraceTypeQuery2" false 0 "None"))
  (if (<= (.Distance (Collision|BreakHitResult _outhit)) 5e+02)
    (AI|Components|Blackboard|SetValueasBool _returnvalue_3 _returnvalue true)
    (else
      (AI|Components|Blackboard|SetValueasBool _returnvalue_3 _returnvalue false))))

(fn ConstructionScript)