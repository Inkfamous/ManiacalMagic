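; Wave spawner that fills a resizable box volume with randomly chosen melee and shooter AI enemies.
; WaveSpawn arms a flag, and the next Tick spawns one batch sized by Limit, adding each enemy to the TopDownGameMode count.
; Spawns use raised random points in the box, with rotation aimed at the player from a separately rolled point.
; The spawner destroys itself if armed once WaveCounter reaches MaxWaves, though it never increments that counter.
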(event Custom|Wave%20Spawn
  (Variables|Default|SetAllow%20Spawning true))

(event EventTick
  (params (DeltaSeconds :type Float%20%28single-precision%29))
  (if (Variables|Default|GetAllow%20Spawning)
    (if (>= (Variables|Default|GetWave%20Counter) (Variables|Default|GetMax%20Waves))
      (Actor|DestroyActor)
      (else
        (for _index (range 0 (Variables|Default|GetLimit))
          (if (== (Math|Random|RandomIntegerinRange 0 1) 0)
            (bind (_location _rotator) (CallFunction|GiveRandomSpawn))
            (CallFunction|SpawnMelee _location _rotator)
            (else
              (bind (_location_2 _rotator_2) (CallFunction|GiveRandomSpawn))
              (CallFunction|SpawnShooter _location_2 _rotator_2)))
          (bind _astop_down_game_mode (Utilities|Casting|CastToTopDownGameMode (Game|GetGameMode)))
          (bind _output_get (Variables|/Game/TopDownBP/Blueprints/TopDownGameMode.TopDownGameMode_C|SetEnemies _astop_down_game_mode (+ (Variables|/Game/TopDownBP/Blueprints/TopDownGameMode.TopDownGameMode_C|GetEnemies _astop_down_game_mode) 1)))
          (Development|PrintString (Utilities|String|ToString(Integer) _output_get)))
        (Variables|Default|SetAllow%20Spawning false)))))

(fn ConstructionScript
  (Components|Box|SetBoxExtent (Variables|Default|GetBox) (Variables|Default|GetBox%20Size) true))

(fn SpawnShooter
  (params (Location :type Vector) (Rotation :type Rotator))
  (bind _shooter (Variables|Default|GetShooter))
  (AI|SpawnAIFromClass (Utilities|Array|Get(acopy) _shooter (Math|Random|RandomIntegerinRange 0 (- (Utilities|Array|Length _shooter) 1))) "/Game/AI/BT_ShooterAI.BT_ShooterAI" Location Rotation false 0))

(fn SpawnMelee
  (params (Location :type Vector) (Rotation :type Rotator))
  (bind _melee (Variables|Default|GetMelee))
  (AI|SpawnAIFromClass (Utilities|Array|Get(acopy) _melee (Math|Random|RandomIntegerinRange 0 (- (Utilities|Array|Length _melee) 1))) "/Game/AI/BT_MeleeAI.BT_MeleeAI" Location Rotation false 0))

(fn GiveRandomSpawn
  (bind _box (Variables|Default|GetBox))
  (bind (_origin _boxextent) (Collision|GetComponentBounds _box))
  (bind _returnvalue (Math|Random|RandomPointinBoundingBox _origin _boxextent))
  (return (+ _returnvalue "0, 0,100.000000") (Math|Rotator|FindLookatRotation _returnvalue (Transformation|GetWorldLocation (Variables|/Script/Engine.Character|GetCapsuleComponent (Game|GetPlayerCharacter 0))))))