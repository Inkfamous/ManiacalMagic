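; BP_ShooterSpawner is a spawner actor that creates ShooterAI enemies running the BT_ShooterAI behavior tree.
; On BeginPlay it caches the player's TopDownCharacter.
; Its WorldSpawn event, which nothing in this graph calls, spawns one AI slightly above the spawner's root, rotated to look at the player's capsule.
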(event Custom|World%20Spawn
  (bind _defaultsceneroot (Variables|Default|GetDefaultSceneRoot))
  (bind _returnvalue (Transformation|GetWorldLocation _defaultsceneroot))
  (AI|SpawnAIFromClass (Variables|Default|GetShooterAI) "/Game/AI/Behavior_Tree/BT_ShooterAI.BT_ShooterAI" (+ _returnvalue "0, 0,100.000000") (Math|Rotator|FindLookatRotation _returnvalue (Transformation|GetWorldLocation (Variables|/Script/Engine.Character|GetCapsuleComponent (Variables|Default|GetTop%20Down%20Character)))) false 0))

(event EventBeginPlay
  (bind _astop_down_character (Utilities|Casting|CastToTopDownCharacter (Game|GetPlayerCharacter 0)))
  (Variables|Default|SetTop%20Down%20Character _astop_down_character))

(fn ConstructionScript)