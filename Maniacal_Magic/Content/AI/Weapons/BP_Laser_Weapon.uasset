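; BP_Laser_Weapon is a short-lived laser beam actor that destroys itself three seconds after spawning.
; The construction script line-traces 2000 units along the spline's forward vector with persistent debug drawing, then stretches a spline mesh between start and end.
; The beam ends at the trace end rather than the impact point, so hits never shorten it.
; Spline overlap casts to TopDownCharacter but applies no effect.
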(event OnComponentBeginOverlap(Spline)
  (params (OverlappedComponent :type Primitive%20Component%20Object%20Reference) (OtherActor :type Actor%20Object%20Reference) (OtherComp :type Primitive%20Component%20Object%20Reference) (OtherBodyIndex :type Integer) (bFromSweep :type Boolean) (SweepResult :type Hit%20Result%20Structure%20%28by%20ref%29))
  (Utilities|Casting|CastToTopDownCharacter OtherActor))

(event EventBeginPlay
  (Utilities|FlowControl|Delay 3.0)
  (Actor|DestroyActor))

(fn ConstructionScript
  (bind _spline (Variables|Default|GetSpline))
  (bind _spline_2 (Variables|Default|GetSpline))
  (bind _spline_3 (Variables|Default|GetSpline))
  (bind _returnvalue (Transformation|GetWorldLocation _spline))
  (bind _outhit (Collision|LineTraceForObjects _returnvalue (+ (* (Math|Vector|GetForwardVector (Transformation|GetWorldRotation _spline)) 2e+03) _returnvalue) (Utilities|Array|MakeArray "ObjectTypeQuery1" "ObjectTypeQuery2") false 0 "Persistent"))
  (Variables|Default|SetStart%20Location _returnvalue)
  (Variables|Default|SetEnd%20Location (.TraceEnd (Collision|BreakHitResult _outhit)))
  (bind _returnvalue_2 (AddComponent|AddSplineMeshComponent false))
  (SplineMesh|SetForwardAxis _returnvalue_2 "Z" true)
  (Spline|SetLocationatSplinePoint _spline_2 0 (Variables|Default|GetStart%20Location) "World" true)
  (Spline|SetLocationatSplinePoint _spline_2 1 (Variables|Default|GetEnd%20Location) "World" true)
  (SplineMesh|SetStartandEnd _returnvalue_2 (Spline|GetLocationatSplinePoint _spline_3 0 "Local") "0, 0, 0" (Spline|GetLocationatSplinePoint _spline_3 1 "Local") "0, 0, 0" true :!class /Script/Engine.SplineMeshComponent))