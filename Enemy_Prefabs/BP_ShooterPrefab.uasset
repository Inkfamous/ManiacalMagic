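; BP_ShooterPrefab is a shooter enemy that tracks player proximity and takes damage.
; BeginPlay starts a looping timer at FireRate calling FireProjectile, which is empty here.
; Sphere overlaps with TopDownCharacter toggle PlayerFound, noted as controlling the AI Behavior Tree.
; Damage reduces Shield first, then Health; below zero Health, it decrements the TopDownGameMode EnemyCount if positive and destroys itself.
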(event OnComponentBeginOverlap(Sphere)
  (params (OverlappedComponent :type Primitive%20Component%20Object%20Reference) (OtherActor :type Actor%20Object%20Reference) (OtherComp :type Primitive%20Component%20Object%20Reference) (OtherBodyIndex :type Integer) (bFromSweep :type Boolean) (SweepResult :type Hit%20Result%20Structure%20%28by%20ref%29))
  ;[0 1 0.9647] Tells the AI Behaviour Tree to fucking stop, and then summarily start again - Nathan
  (Utilities|Casting|CastToTopDownCharacter OtherActor)
  (Variables|Default|SetPlayerFound true))

(event OnComponentEndOverlap(Sphere)
  (params (OverlappedComponent :type Primitive%20Component%20Object%20Reference) (OtherActor :type Actor%20Object%20Reference) (OtherComp :type Primitive%20Component%20Object%20Reference) (OtherBodyIndex :type Integer))
  ;[0 1 0.9647] Tells the AI Behaviour Tree to fucking stop, and then summarily start again - Nathan
  (Utilities|Casting|CastToTopDownCharacter OtherActor)
  (Variables|Default|SetPlayerFound false))

(event Custom|Fire%20Projectile
  ;[0 1 0.9647] Fires a Projectile on a set fire rate - Nathan
)

(event Game|Damage|EventAnyDamage
  (params (Damage :type Float%20%28single-precision%29) (DamageType :type Damage%20Type%20Object%20Reference) (InstigatedBy :type Controller%20Object%20Reference) (DamageCauser :type Actor%20Object%20Reference))
  (bind _returnvalue (Game|GetGameMode))
  (bind _returnvalue_2 (Math|Float|Truncate Damage))
  (bind _astop_down_game_mode (Utilities|Casting|CastToTopDownGameMode _returnvalue))
  (if (> (Variables|Default|GetShield) 0)
    (Variables|Default|SetShield (- (Variables|Default|GetShield) _returnvalue_2))
    (else
      (bind _output_get (Variables|Default|SetHealth (- (Variables|Default|GetHealth) _returnvalue_2)))
      (if (< _output_get 0)
        (if (> (Variables|/Game/TopDownBP/Blueprints/TopDownGameMode.TopDownGameMode_C|GetEnemy%20Count _astop_down_game_mode) 0)
          (Variables|/Game/TopDownBP/Blueprints/TopDownGameMode.TopDownGameMode_C|SetEnemy%20Count _astop_down_game_mode (- (Variables|/Game/TopDownBP/Blueprints/TopDownGameMode.TopDownGameMode_C|GetEnemy%20Count _astop_down_game_mode) 1)))
        (Actor|DestroyActor)))))

(event EventBeginPlay
  ;[0 1 0.9647] Fires a Projectile on a set fire rate - Nathan
  (Utilities|Time|SetTimerbyEvent (delegate Custom|Fire%20Projectile) (Variables|Default|GetFireRate) true))

(fn ConstructionScript)